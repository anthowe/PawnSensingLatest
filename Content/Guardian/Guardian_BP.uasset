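; Guardian is an AI-controlled Blueprint that runs a behavior tree and has an emissive eye with a changeable color.
; On BeginPlay it casts its controller to My_AIC and passes it the behavior tree, with the player pawn as the pawn-sensing target.
; The construction script creates a dynamic emissive material on the Eye, stores it and hands it to a color-changing component.
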(event `self.ReceiveBeginPlay`
  ;[1 1 1] Begin Play
  (bind _asmy_aic (cast `/Game/BT/My_AIC` (`AIBlueprintHelperLibrary.GetAIController` self)))
  (`/Game/BT/My_AIC.Setup_AIC` _asmy_aic (`self.BT`) (`GameplayStatics.GetPlayerPawn` 0)))

(fn `UserConstructionScript`
  ;[1 1 1] SetupDynamicEyeMaterialComponent
  (bind _returnvalue (`PrimitiveComponent.CreateDynamicMaterialInstance` (`self.Eye`) 0 "/Game/Guardian/GenericEmissiveColor.GenericEmissiveColor" "None"))
  (bind _output_get (set `self.DynamicEyeMatColorRef` _returnvalue))
  (`/Game/Guardian/GenericEmissiveColourChangingComponent.Setup` (`self.GenericEmissiveColourChangingComponent`) _output_get))