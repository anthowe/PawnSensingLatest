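; GuardianProjectileBP is a projectile, filed with the Guardian AI, that explodes when its BlockAll collision component hits something.
; Detonate runs once, spawning an explosion emitter and a loud, low-pitched attenuated sound at that component's location, then destroys the actor.
; A LaunchCharacter function can knock a character along the direction from the projectile to a given actor, but nothing in this file calls it.
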(event `self.BlockAll.OnComponentHit`
  (params (HitComponent :type "PrimitiveComponent Object Reference") (OtherActor :type "Actor Object Reference") (OtherComp :type "PrimitiveComponent Object Reference") (NormalImpulse :type "Vector Structure") (Hit :type "HitResult Structure (by ref)"))
  (`self.Detonate`))

(event `self.ProjectileMovement.OnProjectileBounce`
  (params (ImpactResult :type "HitResult Structure (by ref)") (ImpactVelocity :type "Vector Structure (by ref)")))

(event `Detonate`
  (bind _returnvalue (`SceneComponent.K2_GetComponentLocation` (`self.BlockAll`)))
  (`/Engine/EditorBlueprintResources/StandardMacros.DoOnce` false
    (:`Completed`
      (`GameplayStatics.SpawnEmitterAtLocation` "/Game/StarterContent/Particles/P_Explosion.P_Explosion" _returnvalue)
      (`GameplayStatics.PlaySoundAtLocation` "/Game/StarterContent/Audio/Explosion02.Explosion02" _returnvalue (struct) 2.0 0.4 0.0 "/Game/BT/Projectile/MySoundAttenuation.MySoundAttenuation" null null)
      (`self.K2_DestroyActor`))))

(fn `LaunchCharacter`
  (params (Object :type "Object Object Reference") (self2 :type "Actor Object Reference"))
  ;[1 1 1] LaunchCharacter
  (bind _ascharacter (cast `Character` Object))
  (`Character.LaunchCharacter` _ascharacter (* (+ (`KismetMathLibrary.GetDirectionUnitVector` (`SceneComponent.K2_GetComponentLocation` (`self.BlockAll`)) (`self.K2_GetActorLocation` self2)) (0.0 0.0 0.0)) 600.0) false false))

(fn `UserConstructionScript`)